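; BP_DialPuzzle is an interactable puzzle actor that moves the player's camera view to itself when used.
; Interact passes through a DoOnce into a FlipFlop, whose two branches both blend player 0's view target to this actor over a short time.
; ResetInteract re-arms the DoOnce; the graph holds no dial logic and no blend back to the player.
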(event `/Game/Assets/Puzzle/Interfaces/BPI_Interact.Interact`
  (`/Engine/EditorBlueprintResources/StandardMacros.DoOnce` false :!label _label
    (:`Completed`
      (`/Engine/EditorBlueprintResources/StandardMacros.FlipFlop`
        (:`A`
          (`PlayerController.SetViewTargetWithBlend` (`GameplayStatics.GetPlayerController` 0) self 0.3 "VTBlend_Linear" 0.0 false))
        (:`B`
          (`PlayerController.SetViewTargetWithBlend` (`GameplayStatics.GetPlayerController` 0) self 0.3 "VTBlend_Linear" 0.0 false))))))

(event `ResetInteract`
  (goto _label :!via `Reset`))

(fn `UserConstructionScript`
  (`parent.UserConstructionScript`))