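; Base key pickup for the puzzle game, collected when its Interact event fires.
; Interact increments the player's held key count, calls the key count update and crosshair clear on PlayerRef, appends a "None" ID to the held key IDs, then destroys the actor.
; PlayerRef is not assigned in these graphs, and the construction script only calls its parent.
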(event `/Game/Assets/Puzzle/Interfaces/BPI_Interact.Interact`
  (bind _playerref (`self.PlayerRef`))
  (set `/Game/ThirdPerson/Blueprints/BP_FirstPersonCharacter.KeysHeld` (+ (`/Game/ThirdPerson/Blueprints/BP_FirstPersonCharacter.KeysHeld` _playerref) 1) _playerref)
  (`/Game/ThirdPerson/Blueprints/BP_FirstPersonCharacter.UpdateKeysHeld` (`self.PlayerRef`))
  (`/Game/ThirdPerson/Blueprints/BP_FirstPersonCharacter.CrosshairClear` (`self.PlayerRef`))
  (`KismetArrayLibrary.Array_Add` (`/Game/ThirdPerson/Blueprints/BP_FirstPersonCharacter.KeysIDHeld` (`self.PlayerRef`)))
  (`self.K2_DestroyActor`))

(fn `UserConstructionScript`
  (`parent.UserConstructionScript`))