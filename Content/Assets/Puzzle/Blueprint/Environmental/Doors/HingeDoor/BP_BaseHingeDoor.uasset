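; Base hinged door actor that swings open and closed on Interact when its item info marks it as a hinge door.
; With UseDOT, a dot product of door and player orientation picks the swing direction, and the stored angle selects the closing timeline.
; Otherwise fixed open and close timelines rotate the Hinge component's yaw.
; Each swing plays a sound and is locked by a DoOnce until it finishes, when DoorOpen updates.
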(event `/Game/Assets/Puzzle/Interfaces/BPI_Interact.Interact`
  (switch `/Game/Assets/Puzzle/Enum/E_DoorType` (`.DoorType_5_DAAC0885446D121CCF6246B17147E137` (break `/Game/Assets/Puzzle/Struct/S_DoorInfo` (`.DoorInfo_32_08C18C8B43C25D35BD97C49CE39AF909` (break `/Game/Assets/Puzzle/Struct/S_ItemInfo` (`self.ItemInfo`)))))
    (:`NewEnumerator1`
      (if (`self.UseDOT?`)
        (bind _output_get (set `self.Direction` (* (`KismetMathLibrary.Round` (`KismetMathLibrary.Dot_VectorVector` (`KismetMathLibrary.GetForwardVector` (`self.K2_GetActorRotation`)) (`KismetMathLibrary.GetRightVector` (`self.K2_GetActorRotation` (`GameplayStatics.GetPlayerCharacter` 0))))) -1)))
        (if (== _output_get 0)
          _
          (elif (`self.DoorOpen?`)
            (`/Engine/EditorBlueprintResources/StandardMacros.DoOnce` false :!label _label
              (:`Completed`
                (`GameplayStatics.PlaySound2D` null 1.0 1.0 0.0 null null)
                (if (== (`self.DOTDoorAngle`) -90.0)
                  (bind (_direction _doorangle) (`Timeline|Timeline_1` :!via `PlayFromStart`)
                    (:`Update`
                      (`SceneComponent.K2_SetRelativeRotation` (`self.Hinge`) (`KismetMathLibrary.MakeRotator` 0.0 0.0 _doorangle) false false))
                    (:`Finished`
                      (set `self.DoorOpen?` false)
                      (goto _label :!via `Reset`)))
                  (else
                    (bind (_direction_2 _doorangle_2) (`Timeline|Timeline_2` :!via `PlayFromStart`)
                      (:`Update`
                        (`SceneComponent.K2_SetRelativeRotation` (`self.Hinge`) (`KismetMathLibrary.MakeRotator` 0.0 0.0 _doorangle_2) false false))
                      (:`Finished`
                        (set `self.DoorOpen?` false)
                        (goto _label :!via `Reset`)))))))
            (else
              (`/Engine/EditorBlueprintResources/StandardMacros.DoOnce` false :!label _label_2
                (:`Completed`
                  (`GameplayStatics.PlaySound2D` null 1.0 1.0 0.0 null null)
                  (bind (_direction_3 _doorangle_3) (`Timeline|Timeline_0` :!via `PlayFromStart`)
                    (:`Update`
                      (bind _returnvalue (* _doorangle_3 (`self.Direction`)))
                      (set `self.DOTDoorAngle` _returnvalue)
                      (`SceneComponent.K2_SetRelativeRotation` (`self.Hinge`) (`KismetMathLibrary.MakeRotator` 0.0 0.0 _returnvalue) false false))
                    (:`Finished`
                      (set `self.DoorOpen?` true)
                      (goto _label_2 :!via `Reset`))))))))
        (elif (`self.DoorOpen?`)
          (`/Engine/EditorBlueprintResources/StandardMacros.DoOnce` false :!label _label_3
            (:`Completed`
              (`GameplayStatics.PlaySound2D` null 1.0 1.0 0.0 null null)
              (bind (_direction_4 _doorangle_4) (`Timeline|Timeline` :!via `PlayFromStart`)
                (:`Update`
                  (`SceneComponent.K2_SetRelativeRotation` (`self.Hinge`) (`KismetMathLibrary.MakeRotator` 0.0 0.0 _doorangle_4) false false))
                (:`Finished`
                  (set `self.DoorOpen?` false)
                  (goto _label_3 :!via `Reset`)))))
          (else
            (`/Engine/EditorBlueprintResources/StandardMacros.DoOnce` false :!label _label_4
              (:`Completed`
                (`GameplayStatics.PlaySound2D` null 1.0 1.0 0.0 null null)
                (bind (_direction_5 _doorangle_5) (`Timeline|DoorOpen` :!via `PlayFromStart`)
                  (:`Update`
                    (`SceneComponent.K2_SetRelativeRotation` (`self.Hinge`) (`KismetMathLibrary.MakeRotator` 0.0 0.0 _doorangle_5) false false))
                  (:`Finished`
                    (set `self.DoorOpen?` true)
                    (goto _label_4 :!via `Reset`)))))))))))

(fn `UserConstructionScript`
  (`parent.UserConstructionScript`))