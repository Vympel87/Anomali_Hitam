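; BP_BasedItem is an interactable item actor whose data, including mesh, pickup sound and type, comes from a DataTable row.
; The construction script looks up the ItemName row, caches it in ItemInfo and applies its static mesh to the Item component.
; Interact plays the pickup sound in 2D, then switches on the item type, with only the None case wired to destroy the actor.
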(event `/Game/Assets/Puzzle/Dial/Interfaces/BPI_Interact.Interact`
  (bind (_itemclass _staticmesh _itemname _itemdescription _itemtype _itemname_2 _usable_ _pickupsound) (break `/Game/Assets/Puzzle/Dial/Struct/S_ItemInfo` (`self.itemInfo`)))
  (`GameplayStatics.PlaySound2D` _pickupsound 1.0 1.0 0.0 null null)
  (switch `/Game/Assets/Puzzle/Dial/Enum/E_ItemType` _itemtype
    (:`NewEnumerator0`
      (`self.K2_DestroyActor`))))

(fn `UserConstructionScript`
  (bind (_datatable _rowname) (break `DataTableRowHandle` (`self.ItemName`)))
  (bind _returnvalue (`|GetDataTableRow` _datatable _rowname)
    (:`then`
      (bind _output_get (set `self.itemInfo` _returnvalue))
      (`StaticMeshComponent.SetStaticMesh` (`self.Item`) (`.StaticMesh_16_5C73EB24463639686707E0843C5688B7` (break `/Game/Assets/Puzzle/Dial/Struct/S_ItemInfo` _output_get))))))