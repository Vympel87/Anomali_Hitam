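; BP_Base_Enemy is a base enemy that jumpscares the first-person character when it overlaps the enemy's sphere.
; The jumpscare blends the view to the enemy's camera, then plays a sound, camera shake and montage.
; When the montage completes, it returns the view to the player and teleports them to the PlayerStart cached at BeginPlay.
; Patrol points are also cached but unused here, and the AI move-to-player node is unwired.
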(event `self.ReceiveBeginPlay`
  (bind _outactors (`GameplayStatics.GetAllActorsOfClass` "/Game/Enemies/BP_Patrol_Point.BP_Patrol_Point_C"))
  (set `self.PatrolPoint` _outactors)
  (bind _returnvalue (`GameplayStatics.GetActorOfClass` "/Script/Engine.PlayerStart"))
  (set `self.StartPlayer` _returnvalue))

(event `self.Sphere.OnComponentBeginOverlap`
  (params (OverlappedComponent :type "PrimitiveComponent Object Reference") (OtherActor :type "Actor Object Reference") (OtherComp :type "PrimitiveComponent Object Reference") (OtherBodyIndex :type Integer) (bFromSweep :type Boolean) (SweepResult :type "HitResult Structure (by ref)"))
  (cast `/Game/ThirdPerson/Blueprints/BP_FirstPersonCharacter` OtherActor)
  (`self.AI Jumpscare`))

(event `AI Jumpscare`
  (`PlayerController.SetViewTargetWithBlend` (`GameplayStatics.GetPlayerController` 0) (`ActorComponent.GetOwner` (`self.Camera`)) 0.1 "VTBlend_Cubic" 0.0 false)
  (`KismetSystemLibrary.Delay` 0.2)
  (`GameplayStatics.PlaySound2D` null 1.0 1.0 0.0 null null)
  (`GameplayStatics.PlayWorldCameraShake` "/Game/Enemies/BP_CameraShake.BP_CameraShake_C")
  (`|PlayMontage` (`self.Mesh`) "/Game/Characters/Mannequins/Animations/Manny/MM_jumscaare.MM_jumscaare"
    (:`OnCompleted`
      (`KismetSystemLibrary.Delay` 1.0)
      (`PlayerController.SetViewTargetWithBlend` (`GameplayStatics.GetPlayerController` 0) (`GameplayStatics.GetPlayerCharacter` 0) 0.0 "VTBlend_Linear" 0.0 false)
      (bind _returnvalue (`GameplayStatics.GetActorOfClass` "/Game/ThirdPerson/Blueprints/BP_FirstPersonCharacter.BP_FirstPersonCharacter_C"))
      (`PrimitiveComponent.SetSimulatePhysics` (`Character.Mesh` _returnvalue) false)
      (`self.K2_SetActorLocation` (`GameplayStatics.GetPlayerCharacter` 0) (`self.K2_GetActorLocation` (`self.StartPlayer`)) false true))))

(fn `UserConstructionScript`)