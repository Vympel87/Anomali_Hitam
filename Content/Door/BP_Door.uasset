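; Interactive door actor with stepped open states, side detection, sounds and auto-close when the player leaves its trigger box.
; Interaction picks a side by dot product, then a timer advances the state; only the closed case calls HandleDoor.
; HandleRotation ignores its angle, making one interpolation step toward 90 degrees.
; A separate openDoor event drives a timeline swing; Tick is empty, Interact returns false and several interaction checks are unwired.
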(event `self.Box.OnComponentBeginOverlap`
  (params (OverlappedComponent :type "PrimitiveComponent Object Reference") (OtherActor :type "Actor Object Reference") (OtherComp :type "PrimitiveComponent Object Reference") (OtherBodyIndex :type Integer) (bFromSweep :type Boolean) (SweepResult :type "HitResult Structure (by ref)"))
  (if (== OtherActor (`GameplayStatics.GetPlayerCharacter` 0))
    _))

(event `self.ReceiveBeginPlay`
  (bind _asbp_first_person_character (cast `/Game/ThirdPerson/Blueprints/BP_FirstPersonCharacter` (`GameplayStatics.GetPlayerCharacter` 0)))
  (set `self.CharacterRef` _asbp_first_person_character))

(event `self.ReceiveTick`
  (params (DeltaSeconds :type "Float (single-precision)")))

(event `isInteractingWithDoor`
  (params (Player :type "/Game/ThirdPerson/Blueprints/BP_FirstPersonCharacter Object Reference"))
  ;[0 1 0.9727 0.5] Door Interaction Mathematics
  (if (`self.autoCloseActivated?`)
    (set `self.EDoorStates` "NewEnumerator0")
    (set `self.autoClose?` false))
  (`self.Door State Sound`)
  (if (> (`KismetMathLibrary.Dot_VectorVector` (`self.GetActorForwardVector` Player) (`SceneComponent.GetForwardVector` (`self.DoorOpenLocation`))) 0.0)
    (set `self.Door Open Side` 1.0)
    (else
      (set `self.Door Open Side` -1.0)))
  (set `self.bIsInteractingWithDoor` true)
  (`KismetSystemLibrary.K2_SetTimerDelegate` (delegate `CustomEvent`) (`self.Door Sound Time`)))

(event `CustomEvent`
  ;[0 1 0.9727 0.5] Door Interaction Mathematics
  (set `self.bIsInteractingWithDoor` false)
  (switch `/Game/Door/E_DoorState` (`self.EDoorStates`)
    (:`NewEnumerator0`
      (set `self.EDoorStates` "NewEnumerator1")
      (`self.HandleDoor`))
    (:`NewEnumerator1`
      (set `self.EDoorStates` "NewEnumerator2"))
    (:`NewEnumerator2`
      (set `self.EDoorStates` "NewEnumerator0"))))

(event `HandleDoor`
  ;[0.1214 1 0 0.5] Handle Door (Rotating Door According To Door State)
  (switch `/Game/Door/E_DoorState` (`self.EDoorStates`)
    (:`NewEnumerator0`
      (`self.HandleRotation` (* 15.0 (`self.Door Open Side`)))
      (set `self.doorOpen?` true))
    (:`NewEnumerator1`
      (`self.HandleRotation` (* (`self.Door Open Angle`) (`self.Door Open Side`)))
      (set `self.doorOpen?` true))
    (:`NewEnumerator2`
      (if (== (`self.Door Open Side`) 1.0)
        (`self.HandleRotation` -5.0)
        (else
          (`self.HandleRotation` 5.0)))
      (set `self.doorOpen?` false))))

(event `HandleRotation`
  (params (`Set Rotation` :type "Float (double-precision)"))
  (bind _returnvalue (`KismetMathLibrary.MakeRotator` 0.0 0.0 (`KismetMathLibrary.FInterpTo` (.yaw (`SceneComponent.RelativeRotation` (`self.Door`))) 90.0 (`GameplayStatics.GetWorldDeltaSeconds`) (`self.Interp Speed`))))
  ;[1 0.7559 0 0.5] Handle Rotation
  (`SceneComponent.K2_SetRelativeRotation` (`self.Door`) _returnvalue false false)
  (`KismetSystemLibrary.PrintString` (`KismetStringLibrary.Conv_RotatorToString` _returnvalue)))

(event `Door State Sound`
  (bind _returnvalue (`self.K2_GetActorLocation`))
  ;[0 1 0.4189 0.5] Door Sound
  (switch `/Game/Door/E_DoorState` (`self.EDoorStates`)
    (:`NewEnumerator0`
      (`GameplayStatics.PlaySoundAtLocation` "/Game/Door/Audio/Open.Open" _returnvalue (struct) 1.0 1.0 0.0 null null null null))
    (:`NewEnumerator1`
      (`GameplayStatics.PlaySoundAtLocation` "/Game/Door/Audio/partiallyOpen.partiallyOpen" _returnvalue (struct) 1.0 1.0 0.0 null null null null))
    (:`NewEnumerator2`
      (`GameplayStatics.PlaySoundAtLocation` "/Game/Door/Audio/Closed.Closed" _returnvalue (struct) 1.0 1.0 0.0 null null null null))))

(event `self.Box.OnComponentEndOverlap`
  (params (OverlappedComponent :type "PrimitiveComponent Object Reference") (OtherActor :type "Actor Object Reference") (OtherComp :type "PrimitiveComponent Object Reference") (OtherBodyIndex :type Integer))
  (bind _returnvalue (`GameplayStatics.GetPlayerCharacter` 0))
  (bind (_returnvalue_x _returnvalue_y) (`KismetMathLibrary.BreakVector` (`self.GetActorForwardVector` _returnvalue)))
  ;[1 0.2339 0 0.5] Automatic Door Closing
  (set `self.bIsInteractingWithDoor` false)
  (if (and (`self.autoClose?`) (`self.autoClose?`))
    (if (and (== OtherActor _returnvalue) (or (>= _returnvalue_y 0.7) (<= _returnvalue_y -0.7)))
      (`KismetSystemLibrary.Delay` 0.5)
      (`self.Auto Close Door`)
      (set `self.autoCloseActivated?` true))))

(event `Auto Close Door`
  ;[1 0.2339 0 0.5] Automatic Door Closing
  ;;[1 0.2339 0 0.5] Closing Door Functionality
  (`GameplayStatics.PlaySoundAtLocation` "/Game/Door/Audio/Closed.Closed" (`self.K2_GetActorLocation`) (struct) 1.0 1.0 0.0 null null null null)
  (`SceneComponent.K2_SetRelativeRotation` (`self.Door`) (`KismetMathLibrary.MakeRotator` 0.0 0.0 (`KismetMathLibrary.FInterpTo` (.yaw (`SceneComponent.RelativeRotation` (`self.Door`))) 0.0 5.0 (`self.Interp Speed`))) false false))

(event `openDoor`
  (if (`self.doorOpen?`)
    (`KismetSystemLibrary.PrintString` "tutup")
    (bind (_direction _newtrack_0) (`Timeline|Buka Pintu` :!via `Reverse` :!label _label)
      (:`Update`
        (`SceneComponent.K2_SetRelativeRotation` (`self.Door`) (`KismetMathLibrary.MakeRotator` 0.0 0.0 (`KismetMathLibrary.Lerp` 0.0 90.0 _newtrack_0)) false false)
        (`/Engine/EditorBlueprintResources/StandardMacros.DoOnce` false :!label _label_2
          (:`Completed`
            (set `self.doorOpen?` (not (`self.doorOpen?`))))))
      (:`Finished`
        (goto _label_2 :!via `Reset`)))
    (else
      (`KismetSystemLibrary.PrintString` "buka")
      (goto _label :!via `PlayFromStart`))))

(fn `Interact`
  (params (Interactor :type "Character Object Reference"))
  (returns (`Did Interact?` :type Boolean))
  (return false))

(fn `Interact Door`
  (returns (isInteract :type Boolean))
  (return (`self.bIsInteractingWithDoor`)))

(fn `UserConstructionScript`)